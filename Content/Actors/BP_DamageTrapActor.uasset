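; BP_DamageTrapActor is a trap actor that detects overlaps on its DamageVolume but currently only prints debug text, applying no damage.
; BeginPlay binds a custom event to the volume's begin-overlap delegate.
; For a valid overlapping actor, that event passes its display name to PrintName, which prints it and returns whether it is non-empty.
; The event then prints that boolean as a string.
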(event `self.ReceiveBeginPlay`
  (add `PrimitiveComponent.OnComponentBeginOverlap` (`self.DamageVolume`) (delegate `CustomEvent_0`)))

(event `CustomEvent_0`
  (params (OverlappedComponent :type "PrimitiveComponent Object Reference") (OtherActor :type "Actor Object Reference") (OtherComp :type "PrimitiveComponent Object Reference") (OtherBodyIndex :type Integer) (bFromSweep :type Boolean) (SweepResult :type "HitResult Structure (by ref)"))
  (`/Engine/EditorBlueprintResources/StandardMacros.IsValid` OtherActor
    (:`Is Valid`
      (bind _success (`self.PrintName` (`KismetSystemLibrary.GetDisplayName` OtherActor)))
      (`KismetSystemLibrary.PrintString` (`KismetStringLibrary.Conv_BoolToString` _success)))))

(event `self.ReceiveTick`
  (params (DeltaSeconds :type "Float (single-precision)")))

(event `self.OnActorOverlapped`
  (params (Actor :type "Actor Object Reference")))

(fn `PrintName`
  (params (Name :type String))
  (returns (Success :type Boolean))
  (`KismetSystemLibrary.PrintString` Name)
  (if (> (`KismetStringLibrary.Len` Name) 0)
    (return true)
    (else
      (return false))))

(fn `UserConstructionScript`)